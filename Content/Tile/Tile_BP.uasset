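; Endless-runner tile that scrolls along negative X each tick, speeding up with the player's PassedTiles and not scaled by delta time.
; Past the X cutoff it destroys itself, counts the pass if the game has started, and has the GameMode spawn another tile.
; PassedTiles at BeginPlay decides whether Plane28 is a coin pickup, a power-up or removed.
; Tile hits make the player jump; GetAttachTransform exposes the Arrow's transform.
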(event `self.ReceiveBeginPlay`
  (bind _returnvalue_x (`KismetMathLibrary.BreakVector` (`self.K2_GetActorLocation`)))
  (bind _plane28 (`self.Plane28`))
  ;[1 1 1] Begin_Play
  (set `self.Distance_moved` _returnvalue_x)
  (bind _asbp_third_person_character (cast `/Game/ThirdPerson/Blueprints/BP_ThirdPersonCharacter` (`GameplayStatics.GetPlayerCharacter` 0)))
  (bind _passed_tiles (`/Game/ThirdPerson/Blueprints/BP_ThirdPersonCharacter.Passed_Tiles` _asbp_third_person_character))
  (if (== (mod _passed_tiles 5) 0)
    _
    (elif (== (mod _passed_tiles 8) 0)
      (`PrimitiveComponent.SetMaterial` _plane28 0 "/Game/Tile/PowerUpIndicator.PowerUpIndicator")
      (set `self.PowerUp` true)
      (else
        (`ActorComponent.K2_DestroyComponent` _plane28)))))

(event `self.ReceiveTick`
  (params (DeltaSeconds :type "Float (single-precision)"))
  (bind _returnvalue_x (`KismetMathLibrary.BreakVector` (`self.K2_GetActorLocation`)))
  ;[1 1 1] Event TIck
  (bind _asbp_third_person_character (cast `/Game/ThirdPerson/Blueprints/BP_ThirdPersonCharacter` (`GameplayStatics.GetPlayerCharacter` 0)))
  (bind _output_get (set `self.Distance_moved` (- (`self.Distance_moved`) (+ (`self.Speed`) (* (`KismetMathLibrary.Conv_IntToDouble` (`/Game/ThirdPerson/Blueprints/BP_ThirdPersonCharacter.Passed_Tiles` _asbp_third_person_character)) (`self.Acceleration`))))))
  (`self.K2_SetActorTransform` (`KismetMathLibrary.MakeTransform` (`KismetMathLibrary.MakeVector` _output_get)))
  (if (<= _returnvalue_x -2000.0)
    (`self.K2_DestroyActor`)
    (bind _asbp_third_person_game_mode (cast `/Game/ThirdPerson/Blueprints/BP_ThirdPersonGameMode` (`GameplayStatics.GetGameMode`)))
    (if (`/Game/ThirdPerson/Blueprints/BP_ThirdPersonGameMode.IsStarted` _asbp_third_person_game_mode)
      (bind _asbp_third_person_character_2 (cast `/Game/ThirdPerson/Blueprints/BP_ThirdPersonCharacter` (`GameplayStatics.GetPlayerCharacter` 0)))
      (set `/Game/ThirdPerson/Blueprints/BP_ThirdPersonCharacter.Passed_Tiles` (+ (`/Game/ThirdPerson/Blueprints/BP_ThirdPersonCharacter.Passed_Tiles` _asbp_third_person_character_2) 1) _asbp_third_person_character_2))
    (bind _asbp_third_person_game_mode_2 (cast `/Game/ThirdPerson/Blueprints/BP_ThirdPersonGameMode` (`GameplayStatics.GetGameMode`)))
    (`/Game/ThirdPerson/Blueprints/BP_ThirdPersonGameMode.SpawnTile` _asbp_third_person_game_mode_2)))

(event `self.Tile1.OnComponentHit`
  (params (HitComponent :type "PrimitiveComponent Object Reference") (OtherActor :type "Actor Object Reference") (OtherComp :type "PrimitiveComponent Object Reference") (NormalImpulse :type "Vector Structure") (Hit :type "HitResult Structure (by ref)"))
  ;[1 1 1] Bounce_Player
  (bind _asbp_third_person_character (cast `/Game/ThirdPerson/Blueprints/BP_ThirdPersonCharacter` OtherActor))
  (`Character.Jump` _asbp_third_person_character))

(event `self.Tile.OnComponentHit`
  (params (HitComponent :type "PrimitiveComponent Object Reference") (OtherActor :type "Actor Object Reference") (OtherComp :type "PrimitiveComponent Object Reference") (NormalImpulse :type "Vector Structure") (Hit :type "HitResult Structure (by ref)"))
  ;[1 1 1] Bounce_Player
  (bind _asbp_third_person_character (cast `/Game/ThirdPerson/Blueprints/BP_ThirdPersonCharacter` OtherActor))
  (`Character.Jump` _asbp_third_person_character))

(event `self.Plane28.OnComponentBeginOverlap`
  (params (OverlappedComponent :type "PrimitiveComponent Object Reference") (OtherActor :type "Actor Object Reference") (OtherComp :type "PrimitiveComponent Object Reference") (OtherBodyIndex :type Integer) (bFromSweep :type Boolean) (SweepResult :type "HitResult Structure (by ref)"))
  ;[1 1 1] Power_UP_wall
  (`ActorComponent.K2_DestroyComponent` (`self.Plane28`))
  (if (`self.PowerUp`)
    (message `/Game/Tile/PowerUp/PowerUp_Interface.Power Up` OtherActor)
    (set `self.PowerUp` false)
    (else
      (bind _asbp_third_person_character (cast `/Game/ThirdPerson/Blueprints/BP_ThirdPersonCharacter` OtherActor))
      (bind _returnvalue (`GameplayStatics.LoadGameFromSlot` "save1"))
      (cast `/Game/ThirdPerson/Blueprints/BP_Save` _returnvalue)
      (set `/Game/ThirdPerson/Blueprints/BP_ThirdPersonCharacter.TotalCoins` (+ (`/Game/ThirdPerson/Blueprints/BP_ThirdPersonCharacter.TotalCoins` _asbp_third_person_character) (`/Game/ThirdPerson/Blueprints/BP_ThirdPersonCharacter.BaseCoinMulti` _asbp_third_person_character)) _asbp_third_person_character))))

(fn `Get Attach Transform`
  (returns (`Attach Transform` :type "Transform Structure"))
  (return (`SceneComponent.K2_GetComponentToWorld` (`self.Arrow`))))

(fn `Power Up`)

(fn `UserConstructionScript`)